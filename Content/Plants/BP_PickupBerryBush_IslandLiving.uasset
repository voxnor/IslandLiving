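; A harvestable island berry bush that gives up its berry on use and regrows it on a timer.
; On use it spawns a BP_BerryGhost_IslandLiving at its transform and forwards the use to it, presumably to handle the pickup.
; It then hides the Berry component and blocks further use until a timer restores it.
; It is also chainsawable, returning a random stack of berry items.
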(event Custom|CustomEvent
  (Rendering|SetVisibility (Variables|Default|GetBerry) true false)
  (Variables|Default|SetbIsBerryAvailable true))

(event EventBeginPlay)

(event Collision|EventActorBeginOverlap
  (params (OtherActor :type Actor%20Object%20Reference)))

(event EventTick
  (params (DeltaSeconds :type Float%20%28single-precision%29)))

(event EventOnUse
  (params (byCharacter :type FG%20Character%20Player%20Object%20Reference) (state :type Use%20State%20Structure%20%28by%20ref%29))
  (bind _returnvalue (Game|SpawnActorfromClass "/IslandLiving/Plants/BP_BerryGhost_IslandLiving.BP_BerryGhost_IslandLiving_C" (Transformation|GetActorTransform) "AlwaysSpawn" "MultiplyWithRoot" 0 0))
  (Default|TriggerUse _returnvalue byCharacter)
  (Rendering|SetVisibility (Variables|Default|GetBerry) false false)
  (Variables|Default|SetbIsBerryAvailable false)
  (Utilities|Time|SetTimerbyEvent (delegate Custom|CustomEvent) 15.0))

(fn ConstructionScript
  (|CallParentFunction))

(fn IsUseable
  (return (Variables|Default|GetbIsBerryAvailable)))

(fn GetActorChainsawReturn
  (return (Class|FGInventoryLibrary|MakeInventoryStack (Math|Random|RandomIntegerinRange 12 20) (Class|FGInventoryLibrary|MakeInventoryItem "/Game/FactoryGame/Resource/Environment/Berry/Desc_Berry.Desc_Berry_C"))))

(fn GetMeshComponent
  (return (Variables|Default|GetStaticMesh)))

(fn IsChainsawable
  (return true))