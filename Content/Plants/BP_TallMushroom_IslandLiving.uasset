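; BP_TallMushroom_IslandLiving is a tall mushroom plant actor that can be chainsawed to harvest Mycelia.
; It overrides chainsaw functions to expose its static mesh and return a randomly sized stack of Mycelia.
; Its use functions report it as not useable, with an empty look-at description and no interaction blocking.
; The event graph and construction script contain no active logic.
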(event EventBeginPlay)

(event Collision|EventActorBeginOverlap
  (params (OtherActor :type Actor%20Object%20Reference)))

(event EventTick
  (params (DeltaSeconds :type Float%20%28single-precision%29)))

(fn ConstructionScript)

(fn GetActorChainsawReturn
  (return (Class|FGInventoryLibrary|MakeInventoryStack (Math|Random|RandomIntegerinRange 25 45) (Class|FGInventoryLibrary|MakeInventoryItem "/Game/FactoryGame/Resource/Parts/GenericBiomass/Desc_Mycelia.Desc_Mycelia_C"))))

(fn GetLookatDecription
  (params (byCharacter :type FG%20Character%20Player%20Object%20Reference) (state :type Use%20State%20Structure%20%28by%20ref%29))
  (return ""))

(fn GetMeshComponent
  (return (Variables|Default|GetStaticMesh)))

(fn IsChainsawable
  (return true))

(fn IsUseable
  (return false))

(fn ShouldBlockInteraction
  (params (byCharacter :type FG%20Character%20Player%20Object%20Reference) (hitResult :type Hit%20Result%20Structure%20%28by%20ref%29))
  (return false))

(fn UpdateUseState
  (params (byCharacter :type FG%20Character%20Player%20Object%20Reference) (atLocation :type Vector%20%28by%20ref%29 :default "0, 0, 0") (componentHit :type Primitive%20Component%20Object%20Reference) (out_useState :type Use%20State%20Structure%20%28by%20ref%29))
  (return))