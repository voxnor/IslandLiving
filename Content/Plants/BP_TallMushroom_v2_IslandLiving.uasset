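; Blueprint for a living island variant of the tall mushroom plant, which players can chainsaw but not otherwise use.
; It overrides the chainsaw interface to report itself chainsawable, expose its static mesh, and yield a random stack of Mycelia when cut.
; Event graph stubs are disabled and the construction script only calls its parent, so all behavior lives in these overrides.
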(event EventBeginPlay)

(event Collision|EventActorBeginOverlap
  (params (OtherActor :type Actor%20Object%20Reference)))

(event EventTick
  (params (DeltaSeconds :type Float%20%28single-precision%29)))

(fn ConstructionScript
  (|CallParentFunction))

(fn IsUseable
  (return false))

(fn GetActorChainsawReturn
  (return (Class|FGInventoryLibrary|MakeInventoryStack (Math|Random|RandomIntegerinRange 25 45) (Class|FGInventoryLibrary|MakeInventoryItem "/Game/FactoryGame/Resource/Parts/GenericBiomass/Desc_Mycelia.Desc_Mycelia_C"))))

(fn GetMeshComponent
  (return (Variables|Default|GetStaticMesh)))

(fn IsChainsawable
  (return true))