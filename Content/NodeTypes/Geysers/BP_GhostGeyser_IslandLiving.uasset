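; Placeholder "ghost" geyser actor for the IslandLiving mod that spawns or removes a pure geyser node at its own transform.
; SpawnLogic finds an existing BP_GeyserNodePure_IslandLiving by matching GeyserID to GeyserIDParent, then reads the EnableGeysersIL config flag.
; When enabled it spawns a node only if none is found; when disabled it destroys the linked node.
; Nothing in this graph calls SpawnLogic.
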(event EventBeginPlay)

(event Collision|EventActorBeginOverlap
  (params (OtherActor :type Actor%20Object%20Reference)))

(event EventTick
  (params (DeltaSeconds :type Float%20%28single-precision%29)))

(fn ConstructionScript)

(fn SpawnLogic
  (bind _outactors (Actor|GetAllActorsOfClass "/IslandLiving/NodeTypes/Geysers/BP_GeyserNodePure_IslandLiving.BP_GeyserNodePure_IslandLiving_C"))
  (for _array_element _outactors
    (if (== (Variables|/IslandLiving/NodeTypes/Geysers/BP_GeyserNodePure_IslandLiving.BP_GeyserNodePure_IslandLiving_C|GetgeyserID _array_element) (Variables|Default|GetgeyserIDParent))
      (Variables|Default|SetspawnedGeyser _array_element)))
  (bind _asconfig_property_section (Utilities|Casting|CastToConfigPropertySection (Class|RuntimeBlueprintFunctionLibrary|ToConfigProperty(ModConfiguration) "/IslandLiving/IslandLiving_Config.IslandLiving_Config_C")))
  (if (Class|RuntimeBlueprintFunctionLibrary|ToBoolean(ConfigProperty) (Class|RuntimeBlueprintFunctionLibrary|ToConfigProperty(ConfigPropertySection) _asconfig_property_section "EnableGeysersIL"))
    (if (not (Utilities|IsValid (Variables|Default|GetspawnedGeyser)))
      (bind _returnvalue (Game|SpawnActorfromClass "/IslandLiving/NodeTypes/Geysers/BP_GeyserNodePure_IslandLiving.BP_GeyserNodePure_IslandLiving_C" (Transformation|GetActorTransform) "Undefined" "MultiplyWithRoot" 0 (Variables|Default|GetgeyserIDParent) 0))
      (Variables|Default|SetspawnedGeyser _returnvalue))
    (elif (Utilities|IsValid (Variables|Default|GetspawnedGeyser))
      (Default|Destroy (Variables|Default|GetspawnedGeyser))
      (Variables|Default|SetspawnedGeyser 0))))