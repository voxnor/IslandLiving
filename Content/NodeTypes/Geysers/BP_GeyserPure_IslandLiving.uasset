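; BP_GeyserPure_IslandLiving is a geyser resource node variant that provides an infinite, pure-purity geyser resource.
; Construction and BeginPlay both force purity to Pure, and BeginPlay initializes the resource with the geyser descriptor before running parent logic.
; It then assigns the collision mesh to the resource collision component and always reports that it should be saved.
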(event EventBeginPlay
  (Variables|Default|SetmPurity "RP_Pure")
  (Class|FGResourceNode|InitResource "/Game/FactoryGame/Resource/RawResources/Geyser/Desc_Geyser.Desc_Geyser_C" "RA_Infinite" "RP_Pure")
  (|CallParentFunction)
  (Components|StaticMesh|SetStaticMesh (Variables|Default|GetResourceCollision) (Variables|Default|GetCollisionMesh)))

(event Collision|EventActorBeginOverlap
  (params (OtherActor :type Actor%20Object%20Reference)))

(event EventTick
  (params (DeltaSeconds :type Float%20%28single-precision%29)))

(fn ConstructionScript
  (Variables|Default|SetmPurity "RP_Pure")
  (|CallParentFunction))

(fn ShouldSave
  (return true))