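; Spawner actor for the pure bauxite resource node of IslandLiving, placed in the world to create that node at its own transform.
; SpawnLogic scans every existing node of that class and exits if one already carries the same NodeID.
; Otherwise it spawns the node with AlwaysSpawn collision handling and passes its NodeID along, so repeated runs create no duplicates.
; The event graph is unused, and nothing in this file calls SpawnLogic.
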(event EventBeginPlay
  (|CallParentFunction) ; This node is disabled and will not be called.\nDrag off pins to build functionality.
)

(event Collision|EventActorBeginOverlap
  (params (OtherActor :type Actor%20Object%20Reference))
  (|CallParentFunction OtherActor) ; This node is disabled and will not be called.\nDrag off pins to build functionality.
)

(event EventTick
  (params (DeltaSeconds :type Float%20%28single-precision%29))
  (|CallParentFunction DeltaSeconds) ; This node is disabled and will not be called.\nDrag off pins to build functionality.
)

(fn ConstructionScript
  (|CallParentFunction))

(fn SpawnLogic
  (bind _outactors (Actor|GetAllActorsOfClass "/IslandLiving/NodeTypes/Bauxite/BP_ResourceNode_BauxitePure_IslandLiving.BP_ResourceNode_BauxitePure_IslandLiving_C"))
  (for _array_element _outactors
    (if (== (Variables|/IslandLiving/BP_ResourceNode_IslandLiving.BP_ResourceNode_IslandLiving_C|GetNodeID _array_element) (Variables|Default|GetNodeID))
      (return)))
  (Game|SpawnActorfromClass "/IslandLiving/NodeTypes/Bauxite/BP_ResourceNode_BauxitePure_IslandLiving.BP_ResourceNode_BauxitePure_IslandLiving_C" (Transformation|GetActorTransform) "AlwaysSpawn" "MultiplyWithRoot" 0 (Variables|Default|GetNodeID) 0)
  (return))