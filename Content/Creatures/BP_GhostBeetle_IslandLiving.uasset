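; BP_GhostBeetle_IslandLiving is a placeholder that manages one island-living beetle creature, matched by BeetleID.
; SpawnLogic scans existing BP_CreatureBeetle_IslandLiving actors to re-link the one with the same ID.
; The EnableBeetlesIL config toggle then decides whether it spawns a missing beetle at its own transform or destroys the existing one.
; Its event graph is empty, so nothing here calls SpawnLogic.
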(event EventBeginPlay)

(event Collision|EventActorBeginOverlap
  (params (OtherActor :type Actor%20Object%20Reference)))

(event EventTick
  (params (DeltaSeconds :type Float%20%28single-precision%29)))

(fn ConstructionScript)

(fn SpawnLogic
  (bind _outactors (Actor|GetAllActorsOfClass "/IslandLiving/Creatures/BP_CreatureBeetle_IslandLiving.BP_CreatureBeetle_IslandLiving_C"))
  (for _array_element _outactors
    (if (== (Variables|/IslandLiving/Creatures/BP_CreatureBeetle_IslandLiving.BP_CreatureBeetle_IslandLiving_C|GetBeetleID _array_element) (Variables|Default|GetBeetleID))
      (Variables|Default|SetSpawnedCreature _array_element)))
  (bind _asconfig_property_section (Utilities|Casting|CastToConfigPropertySection (Class|RuntimeBlueprintFunctionLibrary|ToConfigProperty(ModConfiguration) "/IslandLiving/IslandLiving_Config.IslandLiving_Config_C")))
  (if (Class|RuntimeBlueprintFunctionLibrary|ToBoolean(ConfigProperty) (Class|RuntimeBlueprintFunctionLibrary|ToConfigProperty(ConfigPropertySection) _asconfig_property_section "EnableBeetlesIL"))
    (if (not (Utilities|IsValid (Variables|Default|GetSpawnedCreature)))
      (bind _returnvalue (Game|SpawnActorfromClass "/IslandLiving/Creatures/BP_CreatureBeetle_IslandLiving.BP_CreatureBeetle_IslandLiving_C" (Transformation|GetActorTransform) "Undefined" "MultiplyWithRoot" 0 (Variables|Default|GetBeetleID) 0))
      (Variables|Default|SetSpawnedCreature _returnvalue))
    (elif (Utilities|IsValid (Variables|Default|GetSpawnedCreature))
      (Default|Destroy (Variables|Default|GetSpawnedCreature))
      (Variables|Default|SetSpawnedCreature 0))))