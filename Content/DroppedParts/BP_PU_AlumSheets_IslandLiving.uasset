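; Dropped-part actor, by its name an aluminum sheets pickup for Island Living, whose presence in the world is toggled by the mod configuration.
; On BeginPlay it reads the EnableDropsIL flag from IslandLiving_Config, enabling collision and showing the actor when true, or disabling collision and hiding it otherwise.
; The actor is never destroyed, and construction only calls the parent script.
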(event EventBeginPlay
  (bind _asconfig_property_section (Utilities|Casting|CastToConfigPropertySection (Class|RuntimeBlueprintFunctionLibrary|ToConfigProperty(ModConfiguration) "/IslandLiving/IslandLiving_Config.IslandLiving_Config_C")))
  (if (Class|RuntimeBlueprintFunctionLibrary|ToBoolean(ConfigProperty) (Class|RuntimeBlueprintFunctionLibrary|ToConfigProperty(ConfigPropertySection) _asconfig_property_section "EnableDropsIL"))
    (Collision|SetActorEnableCollision true)
    (Rendering|SetActorHiddenInGame false)
    (else
      (Collision|SetActorEnableCollision false)
      (Rendering|SetActorHiddenInGame true))))

(event Collision|EventActorBeginOverlap
  (params (OtherActor :type Actor%20Object%20Reference)))

(event EventTick
  (params (DeltaSeconds :type Float%20%28single-precision%29)))

(fn ConstructionScript
  (|CallParentFunction))